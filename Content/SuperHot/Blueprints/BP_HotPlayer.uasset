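; BP_HotPlayer is the player pawn for the SuperHot game, handling input setup and pistol firing.
; BeginPlay adds the IMC_HotInput Enhanced Input mapping context and caches the BP_Pistol from the Pistol child actor component.
; IA_Fire calls Fire on that pistol, gated by a FireDelayed flag and short delay that cap the fire rate.
; Tick is empty, and a time dilation debug print is left disconnected.
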(event Input|EnhancedActionEvents|EnhancedInputActionIA_Fire
  (params (ActionValue :type Boolean) (ElapsedSeconds :type Float%20%28double-precision%29) (TriggeredSeconds :type Float%20%28double-precision%29) (InputAction :type Input%20Action%20Object%20Reference :default "/Game/SuperHot/Inputs/IA_Fire.IA_Fire"))
  (:Triggered
    (if (not (Variables|Default|GetfireDelayed))
      (Variables|Default|SetfireDelayed true)
      (Class|Pistol|Fire (Variables|Default|GetAs%20BP%20Pistol))
      (Utilities|FlowControl|Delay 0.2)
      (Variables|Default|SetfireDelayed false))))

(event EventBeginPlay
  (bind _asplayer_controller (Utilities|Casting|CastToPlayerController (Pawn|GetController)))
  (Utilities|IsValid (PlayerController|LocalPlayerSubsystems|GetEnhancedInputLocalPlayerSubsystem _asplayer_controller)
    (:Is%20Valid
      (Input|AddMappingContext (PlayerController|LocalPlayerSubsystems|GetEnhancedInputLocalPlayerSubsystem _asplayer_controller) "/Game/SuperHot/Inputs/IMC_HotInput.IMC_HotInput" 0 "(bIgnoreAllPressedKeysUntilRelease=True,bForceImmediately=False)")
      (bind _asbp_pistol (Utilities|Casting|CastToBP_Pistol (Variables|/Script/Engine.ChildActorComponent|GetChildActor (Variables|Default|Getpistol))))
      (Variables|Default|SetAs%20BP%20Pistol _asbp_pistol)
      (Variables|Default|SetfireDelayed false))))

(event Collision|EventActorBeginOverlap
  (params (OtherActor :type Actor%20Object%20Reference)))

(event EventTick
  (params (DeltaSeconds :type Float%20%28single-precision%29)))

(fn ConstructionScript)